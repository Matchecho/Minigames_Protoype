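; BP_Pickup is an interactable actor with a flickering point light that prints a success message and destroys itself on Interact.
; A Flickering timeline drives the light intensity between zero and MaxIntensity.
; Tick polls the player's flashlight flag, switching the light off and stopping the timeline while it is set, and playing the timeline otherwise.
; GetInteractText supplies the interaction text.
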(event EventBeginPlay
  (bind _value (Timeline|Flickering Play)
    (:Update
      (Rendering|Components|Light|SetIntensity (Variables|Default|GetPointLight) (Math|Float|Lerp 0.0 (Variables|Default|GetMaxIntensity) _value)))))

(event EventTick
  (params (DeltaSeconds :type Float%20%28single-precision%29))
  (if (Variables|/Game/FirstPersonBP/Blueprints/FirstPersonCharacter.FirstPersonCharacter_C|GetbIsFlashLight (Variables|Default|GetPlayer%20Ref))
    (Rendering|Components|Light|SetIntensity (Variables|Default|GetPointLight) 0.0)
    (bind _value (Timeline|Flickering Stop)
      (:Update
        (Rendering|Components|Light|SetIntensity (Variables|Default|GetPointLight) (Math|Float|Lerp 0.0 (Variables|Default|GetMaxIntensity) _value))))
    (else
      (Timeline|Flickering Play))))

(event EventInteract
  (params (Instigator :type Actor%20Object%20Reference))
  (Development|PrintString "Success")
  (Actor|DestroyActor))

(fn ConstructionScript)

(fn GetInteractText
  (return (Variables|Default|GetText)))