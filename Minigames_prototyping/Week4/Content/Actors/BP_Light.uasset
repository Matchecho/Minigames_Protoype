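; BP_Light is a light actor whose PointLight is shown or hidden through LightOn and LightOff events.
; When IsWithTrigger is set, it starts off at BeginPlay and Tick leaves it alone.
; Otherwise, Tick polls the player's IsFlashLight flag every frame and keeps the light in the opposite state, off while the flashlight flag is true.
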(event Custom|Light%20On
  (Rendering|SetVisibility (Variables|Default|GetPointLight) true false))

(event Custom|Light%20Off
  (Rendering|SetVisibility (Variables|Default|GetPointLight) false false))

(event EventTick
  (params (DeltaSeconds :type Float%20%28single-precision%29))
  (if (not (Variables|Default|GetisWithTrigger))
    (if (Variables|/Game/FirstPersonBP/Blueprints/FirstPersonCharacter.FirstPersonCharacter_C|GetbIsFlashLight (Variables|Default|GetPlayer%20Ref))
      (CallFunction|LightOff)
      (else
        (CallFunction|Lighton)))))

(event EventBeginPlay
  (if (Variables|Default|GetisWithTrigger)
    (CallFunction|LightOff)))

(fn ConstructionScript)