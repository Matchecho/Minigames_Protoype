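; BP_Flickered is an actor that drives a flickering point light.
; On BeginPlay it plays the Flicker timeline, whose value interpolates the PointLight intensity between zero and B on each update.
; An unconnected loop that switches the light on and off with random delays remains in the graph but never runs.
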(event EventBeginPlay
  (bind _value (Timeline|Flicker Play)
    (:Update
      (Rendering|Components|Light|SetIntensity (Variables|Default|GetPointLight) (Math|Float|Lerp 0.0 (Variables|Default|GetB) _value)))))

(fn ConstructionScript)