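; BP_Platform is a platform actor that moves its Hinge back and forth between Closed and Open transforms.
; BeginPlay starts timeline LíneaDeTiempo1, whose Update lerps the Hinge and feeds a three-second Delay that toggles IsOpen to alternate play and reverse.
; Separate OpenDoor and CloseDoor events drive the same Hinge through timeline 1Second.
; The automatic loop sets play rates on 1Second, not on its own timeline.
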(event Custom|Close%20Door
  (Development|PrintString "Door Closed" true true "(R=1.000000,G=0.673725,B=0.000000,A=1.000000)")
  (Components|Timeline|SetPlayRate (Variables|Default|Get1Second) (Variables|Default|GetfClosedDoorRate))
  (Variables|Default|SetbIsOpen false)
  (bind _fvalue (Timeline|1Second Reverse)
    (:Update
      (Transformation|SetRelativeTransform (Variables|Default|GetHinge) (Math|Transform|Lerp(Transform) (Transformation|GetRelativeTransform (Variables|Default|GetClosed)) (Transformation|GetRelativeTransform (Variables|Default|GetOpen)) _fvalue) false false))))

(event Custom|Open%20Door
  (Development|PrintString "Door Opened" true true "(R=1.000000,G=0.673725,B=0.000000,A=1.000000)")
  (Components|Timeline|SetPlayRate (Variables|Default|Get1Second) (Variables|Default|GetfOpenDoorRate))
  (Variables|Default|SetbIsOpen true)
  (bind _fvalue (Timeline|1Second Play)
    (:Update
      (Transformation|SetRelativeTransform (Variables|Default|GetHinge) (Math|Transform|Lerp(Transform) (Transformation|GetRelativeTransform (Variables|Default|GetClosed)) (Transformation|GetRelativeTransform (Variables|Default|GetOpen)) _fvalue) false false))))

(event EventBeginPlay
  (bind _1second (Variables|Default|Get1Second))
  (Components|Timeline|SetPlayRate _1second (Variables|Default|GetfOpenDoorRate) :!label _label)
  (bind _fvalue (Timeline|Línea%20de%20tiempo1 Play)
    (:Update
      (Transformation|SetRelativeTransform (Variables|Default|GetHinge) (Math|Transform|Lerp(Transform) (Transformation|GetRelativeTransform (Variables|Default|GetClosed)) (Transformation|GetRelativeTransform (Variables|Default|GetOpen)) _fvalue) false false)
      (Utilities|FlowControl|Delay 3.0)
      (if (Variables|Default|GetbIsOpen)
        (Variables|Default|SetbIsOpen false)
        (goto _label)
        (else
          (Variables|Default|SetbIsOpen true)
          (Components|Timeline|SetPlayRate _1second (Variables|Default|GetfClosedDoorRate))
          (Timeline|Línea%20de%20tiempo1 Reverse))))))

(fn ConstructionScript)