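; BP_Follower is an enemy character that freezes while the player's flashlight is on and fails the player on contact.
; Tick reads IsFlashLight from the cached FirstPersonCharacter, toggling walk speed and pausing or resuming its sound.
; Overlapping the Grab component forces that flag on, halting the follower, shows the HUD failure state and reloads the current level after a delay.
; No pursuit logic appears in this graph.
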(event OnComponentBeginOverlap(Grab)
  (params (OverlappedComponent :type Primitive%20Component%20Object%20Reference) (OtherActor :type Actor%20Object%20Reference) (OtherComp :type Primitive%20Component%20Object%20Reference) (OtherBodyIndex :type Integer) (bFromSweep :type Boolean) (SweepResult :type Hit%20Result%20Structure%20%28by%20ref%29))
  (bind _asfirst_person_character (Utilities|Casting|CastToFirstPersonCharacter OtherActor))
  (Variables|/Game/FirstPersonBP/Blueprints/FirstPersonCharacter.FirstPersonCharacter_C|SetbIsFlashLight _asfirst_person_character true)
  (Default|SetFailure (Variables|/Game/FirstPersonBP/Blueprints/FirstPersonCharacter.FirstPersonCharacter_C|GetHUD _asfirst_person_character))
  (Utilities|FlowControl|Delay 5.0)
  (bind _returnvalue (Game|GetCurrentLevelName true))
  (Game|OpenLevel(byName) (Utilities|String|StringToName _returnvalue)))

(event EventBeginPlay
  (bind _asfirst_person_character (Utilities|Casting|CastToFirstPersonCharacter (Game|Player|GetPlayerPawn 0)))
  (Variables|Default|SetPlayer%20Ref _asfirst_person_character))

(event EventTick
  (params (DeltaSeconds :type Float%20%28single-precision%29))
  (bind _charactermovement (Variables|Character|GetCharacterMovement))
  (bind _soundeffect (Variables|Default|GetSoundEffect))
  (if (Variables|/Game/FirstPersonBP/Blueprints/FirstPersonCharacter.FirstPersonCharacter_C|GetbIsFlashLight (Variables|Default|GetPlayer%20Ref))
    (Variables|/Script/Engine.CharacterMovementComponent|SetMaxWalkSpeed _charactermovement 0.0)
    (Class|AudioComponent|SetPaused _soundeffect true)
    (else
      (Variables|/Script/Engine.CharacterMovementComponent|SetMaxWalkSpeed _charactermovement 1.5e+02)
      (Class|AudioComponent|SetPaused _soundeffect false))))

(fn ConstructionScript)