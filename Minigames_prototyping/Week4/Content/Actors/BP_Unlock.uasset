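; BP_Unlock is a trigger box that gates a door behind a set of triggers for the first-person character.
; On overlap it opens the door if Openable; otherwise it counts pressed Triggers up to the first unpressed one, never resetting the counter.
; A count matching the array length sets Openable without opening the door; otherwise the HUD shows a hint.
; Leaving the box closes the door when Openable.
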(event OnComponentBeginOverlap(Box)
  (params (OverlappedComponent :type Primitive%20Component%20Object%20Reference) (OtherActor :type Actor%20Object%20Reference) (OtherComp :type Primitive%20Component%20Object%20Reference) (OtherBodyIndex :type Integer) (bFromSweep :type Boolean) (SweepResult :type Hit%20Result%20Structure%20%28by%20ref%29))
  (bind _triggers (Variables|Default|GetTriggers))
  (bind _asfirst_person_character (Utilities|Casting|CastToFirstPersonCharacter OtherActor))
  (if (Variables|Default|GetOpenable)
    (Default|OpenDoor (Variables|Default|GetaDoor))
    (else
      (bind _array_element (Utilities|Array|ForEachLoopwithBreak _triggers :!label _label)
        (:LoopBody
          (if (Variables|/Game/Actors/BP_TriggerText.BP_TriggerText_C|GetPressed _array_element)
            (Variables|Default|SetCounter (+ (Variables|Default|GetCounter) 1))
            (else
              (goto _label Break))))
        (:Completed
          (if (== (Variables|Default|GetCounter) (Utilities|Array|Length _triggers))
            (Variables|Default|SetOpenable true)
            (else
              (Default|SetText (Variables|/Game/FirstPersonBP/Blueprints/FirstPersonCharacter.FirstPersonCharacter_C|GetHUD _asfirst_person_character) "Pressed all the triggers to open the door" (Variables|Default|GetF%20Display%20Time)))))))))

(event OnComponentEndOverlap(Box)
  (params (OverlappedComponent :type Primitive%20Component%20Object%20Reference) (OtherActor :type Actor%20Object%20Reference) (OtherComp :type Primitive%20Component%20Object%20Reference) (OtherBodyIndex :type Integer))
  (Utilities|Casting|CastToFirstPersonCharacter OtherActor)
  (if (Variables|Default|GetOpenable)
    (Default|CloseDoor (Variables|Default|GetaDoor))))

(fn ConstructionScript)