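; Door actor that swings open and closed through OpenDoor and CloseDoor events, which are not triggered within this Blueprint.
; A single timeline plays forward to open and reverses to close, with a separate play rate for each direction.
; Its updates lerp the Hinge's relative transform between the Closed and Open components.
; Both events update IsOpen, while IsPressed is only ever set true, on opening.
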(event Custom|Close%20Door
  (Components|Timeline|SetPlayRate (Variables|Default|Get1Second) (Variables|Default|GetF%20Closed%20Door%20Rate))
  (Variables|Default|SetbIsOpen false)
  (bind _f_value (Timeline|1second Reverse)
    (:Update
      (Transformation|SetRelativeTransform (Variables|Default|GetHinge) (Math|Transform|Lerp(Transform) (Transformation|GetRelativeTransform (Variables|Default|GetClosed)) (Transformation|GetRelativeTransform (Variables|Default|GetOpen)) _f_value) false false))))

(event Custom|Open%20Door
  (Variables|Default|SetbIsPressed true)
  (Components|Timeline|SetPlayRate (Variables|Default|Get1Second) (Variables|Default|GetF%20Open%20Door%20Rate))
  (Variables|Default|SetbIsOpen true)
  (bind _f_value (Timeline|1second Play)
    (:Update
      (Transformation|SetRelativeTransform (Variables|Default|GetHinge) (Math|Transform|Lerp(Transform) (Transformation|GetRelativeTransform (Variables|Default|GetClosed)) (Transformation|GetRelativeTransform (Variables|Default|GetOpen)) _f_value) false false))))

(fn ConstructionScript)