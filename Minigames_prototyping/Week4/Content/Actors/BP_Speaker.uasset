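; BP_Speaker is an actor that plays a sound effect in the world and silences it while the player's flashlight is on.
; It starts the sound on BeginPlay, then checks the PlayerRef flashlight flag every Tick and calls TurnOff or TurnOn.
; Those events pause or unpause the audio component, so playback resumes from where it stopped.
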(event Custom|TurnOff
  (Class|AudioComponent|SetPaused (Variables|Default|GetSoundEffect) true))

(event Custom|TurnOn
  (Class|AudioComponent|SetPaused (Variables|Default|GetSoundEffect) false))

(event EventBeginPlay
  (Audio|Components|Audio|Play (Variables|Default|GetSoundEffect) 0.0))

(event EventTick
  (params (DeltaSeconds :type Float%20%28single-precision%29))
  (if (Variables|/Game/FirstPersonBP/Blueprints/FirstPersonCharacter.FirstPersonCharacter_C|GetbIsFlashLight (Variables|Default|GetPlayerRef))
    (CallFunction|TurnOff)
    (else
      (CallFunction|Turnon))))

(fn ConstructionScript)