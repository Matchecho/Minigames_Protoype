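; BP_Door is a door actor that animates open and closed through OpenDoor and CloseDoor events.
; Each event sets the IsOpen flag and its own play rate on the 1Second timeline, then plays it forward or in reverse.
; Timeline updates lerp the Hinge's relative transform between those of the Closed and Open components, so those components define the two end poses.
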(event Custom|Close%20Door
  (Components|Timeline|SetPlayRate (Variables|Default|Get1Second) (Variables|Default|GetfClosedDoorRate))
  (Variables|Default|SetbIsOpen false)
  (bind _fvalue (Timeline|1Second Reverse)
    (:Update
      (Transformation|SetRelativeTransform (Variables|Default|GetHinge) (Math|Transform|Lerp(Transform) (Transformation|GetRelativeTransform (Variables|Default|GetClosed)) (Transformation|GetRelativeTransform (Variables|Default|GetOpen)) _fvalue) false false))))

(event Custom|Open%20Door
  (Components|Timeline|SetPlayRate (Variables|Default|Get1Second) (Variables|Default|GetfOpenDoorRate))
  (Variables|Default|SetbIsOpen true)
  (bind _fvalue (Timeline|1Second Play)
    (:Update
      (Transformation|SetRelativeTransform (Variables|Default|GetHinge) (Math|Transform|Lerp(Transform) (Transformation|GetRelativeTransform (Variables|Default|GetClosed)) (Transformation|GetRelativeTransform (Variables|Default|GetOpen)) _fvalue) false false))))

(fn ConstructionScript)